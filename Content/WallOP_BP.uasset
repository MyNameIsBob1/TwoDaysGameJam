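; WallOP_BP is a wall actor that penalizes a ThirdPersonCharacter touching it by shortening its FireRange and raising its Heat.
; On BeginPlay it randomly picks one of two meshes and resizes the trigger box to match, tall for one and short for the other.
; The taller variant also rescales the mesh and shifts it along world Y.
; Each box overlap applies the penalty directly to the character's variables.
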(event `self.Box.OnComponentBeginOverlap`
  (params (OverlappedComponent :type "PrimitiveComponent Object Reference") (OtherActor :type "Actor Object Reference") (OtherComp :type "PrimitiveComponent Object Reference") (OtherBodyIndex :type Integer) (bFromSweep :type Boolean) (SweepResult :type "HitResult Structure (by ref)"))
  (bind _asthird_person_character (cast `/Game/ThirdPersonBP/Blueprints/ThirdPersonCharacter` OtherActor))
  (set `/Game/ThirdPersonBP/Blueprints/ThirdPersonCharacter.FireRange` (- (`/Game/ThirdPersonBP/Blueprints/ThirdPersonCharacter.FireRange` _asthird_person_character) (500.0 0.0 0.0)) _asthird_person_character)
  (set `/Game/ThirdPersonBP/Blueprints/ThirdPersonCharacter.Heat` (+ (`/Game/ThirdPersonBP/Blueprints/ThirdPersonCharacter.Heat` _asthird_person_character) 0.25) _asthird_person_character))

(event `self.ReceiveBeginPlay`
  (bind _staticmesh (`self.StaticMesh`))
  (switch `int` (`KismetMathLibrary.RandomIntegerInRange` 0 1)
    (:`0`
      (`SceneComponent.SetWorldScale3D` _staticmesh (6.666667 6.666667 6.666667))
      (`StaticMeshComponent.SetStaticMesh` _staticmesh "/Game/ThirdPersonBP/Box001.Box001")
      (`BoxComponent.SetBoxExtent` (`self.Box`) (337.027588 22.624617 564.160889) true)
      (`SceneComponent.K2_SetWorldLocation` _staticmesh (+ (`SceneComponent.K2_GetComponentLocation` _staticmesh) (0.0 333.0 0.0)) false false))
    (:`1`
      (`StaticMeshComponent.SetStaticMesh` _staticmesh "/Game/ThirdPersonBP/Box002.Box002")
      (`BoxComponent.SetBoxExtent` (`self.Box`) (337.027588 22.624617 56.416088) true))))

(fn `UserConstructionScript`)