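; Self-spawning track tile that chains a path ahead of the player and fills it with random obstacles.
; Player overlap with SpawnBox spawns the next tile at SpawnPoint, sometimes offset along X to leave a gap, while GrabgeCoolect overlap destroys this tile.
; On BeginPlay, each of four point triplets gets one or two SpawnOP calls, each placing a wall at one point and occasionally Ice_BP within Rnad's bounds.
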(event `self.SpawnBox.OnComponentBeginOverlap`
  (params (OverlappedComponent :type "PrimitiveComponent Object Reference") (OtherActor :type "Actor Object Reference") (OtherComp :type "PrimitiveComponent Object Reference") (OtherBodyIndex :type Integer) (bFromSweep :type Boolean) (SweepResult :type "HitResult Structure (by ref)"))
  (bind _returnvalue (`SceneComponent.K2_GetComponentLocation` (`self.SpawnPoint`)))
  (if (== OtherActor (`GameplayStatics.GetPlayerPawn` 0))
    (switch `int` (`KismetMathLibrary.RandomIntegerInRange` 0 4)
      (:`0`
        (`|SpawnActorFromClass` "Tile_BP_C" (`KismetMathLibrary.MakeTransform` _returnvalue) "Undefined" "OverrideRootScale" null null :!label _label))
      (:`1`
        (goto _label))
      (:`2`
        (goto _label))
      (:`3`
        (`|SpawnActorFromClass` "Tile_BP_C" (`KismetMathLibrary.MakeTransform` (+ _returnvalue (300.0 0.0 0.0))) "Undefined" "OverrideRootScale" null null :!label _label_2))
      (:`4`
        (goto _label_2)))))

(event `self.Grabge Coolect.OnComponentBeginOverlap`
  (params (OverlappedComponent :type "PrimitiveComponent Object Reference") (OtherActor :type "Actor Object Reference") (OtherComp :type "PrimitiveComponent Object Reference") (OtherBodyIndex :type Integer) (bFromSweep :type Boolean) (SweepResult :type "HitResult Structure (by ref)"))
  (if (== OtherActor (`GameplayStatics.GetPlayerPawn` 0))
    (`self.K2_DestroyActor`)))

(event `self.ReceiveBeginPlay`
  (`|ExecutionSequence`
    (:`then_0`
      (for _ (range (+ (`KismetMathLibrary.RandomIntegerInRange` 0 1) 1))
        (`self.SpawnOP` (`SceneComponent.K2_GetComponentLocation` (`self.1`)) (`SceneComponent.K2_GetComponentLocation` (`self.2`)) (`SceneComponent.K2_GetComponentLocation` (`self.3`)))))
    (:`then_1`
      (for _ (range (+ (`KismetMathLibrary.RandomIntegerInRange` 0 1) 1))
        (`self.SpawnOP` (`SceneComponent.K2_GetComponentLocation` (`self.4`)) (`SceneComponent.K2_GetComponentLocation` (`self.5`)) (`SceneComponent.K2_GetComponentLocation` (`self.6`)))))
    (:`then_2`
      (for _ (range (+ (`KismetMathLibrary.RandomIntegerInRange` 0 1) 1))
        (`self.SpawnOP` (`SceneComponent.K2_GetComponentLocation` (`self.7`)) (`SceneComponent.K2_GetComponentLocation` (`self.8`)) (`SceneComponent.K2_GetComponentLocation` (`self.9`)))))
    (:`then_3`
      (for _ (range (+ (`KismetMathLibrary.RandomIntegerInRange` 0 1) 1))
        (`self.SpawnOP` (`SceneComponent.K2_GetComponentLocation` (`self.10`)) (`SceneComponent.K2_GetComponentLocation` (`self.11`)) (`SceneComponent.K2_GetComponentLocation` (`self.12`)))))))

(fn `SpawnOP`
  (params (NewParam :type "Vector Structure") (NewParam1 :type "Vector Structure") (NewParam2 :type "Vector Structure"))
  (bind _rnad (`self.Rnad`))
  (switch `int` (`KismetMathLibrary.RandomIntegerInRange` 0 2)
    (:`0`
      (`|SpawnActorFromClass` "/Game/WallOP_BP.WallOP_BP_C" (`KismetMathLibrary.MakeTransform` NewParam) "Undefined" "OverrideRootScale" null null))
    (:`1`
      (`|SpawnActorFromClass` "/Game/WallOP_BP.WallOP_BP_C" (`KismetMathLibrary.MakeTransform` (- NewParam1 (0.0 333.0 0.0))) "Undefined" "OverrideRootScale" null null))
    (:`2`
      (`|SpawnActorFromClass` "/Game/WallOP_BP.WallOP_BP_C" (`KismetMathLibrary.MakeTransform` (+ NewParam2 (0.0 333.0 0.0))) "Undefined" "OverrideRootScale" null null)))
  (switch `int` (`KismetMathLibrary.RandomIntegerInRange` 0 15)
    (:`0`
      (`|SpawnActorFromClass` "/Game/Ice_BP.Ice_BP_C" (`KismetMathLibrary.MakeTransform` (`KismetMathLibrary.RandomPointInBoundingBox` (`SceneComponent.K2_GetComponentLocation` _rnad) (`BoxComponent.BoxExtent` _rnad))) "Undefined" "OverrideRootScale" null null))))

(fn `UserConstructionScript`)