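; Ice pickup actor that modifies the ThirdPersonCharacter's fire range and heat when collected.
; Tick spins it continuously around the yaw axis at a configurable turn speed, scaled by delta time.
; When a ThirdPersonCharacter overlaps its box, it extends FireRange along X, lowers Heat by a fixed amount and destroys itself.
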(event `self.ReceiveTick`
  (params (DeltaSeconds :type "Float (single-precision)"))
  (bind (_returnvalue_roll _returnvalue_pitch _returnvalue_yaw) (`KismetMathLibrary.BreakRotator` (`self.K2_GetActorRotation`)))
  (`self.K2_SetActorRotation` (`KismetMathLibrary.MakeRotator` _returnvalue_roll _returnvalue_pitch (+ (* (`self.TrunSpeed`) DeltaSeconds) _returnvalue_yaw)) true))

(event `self.Box.OnComponentBeginOverlap`
  (params (OverlappedComponent :type "PrimitiveComponent Object Reference") (OtherActor :type "Actor Object Reference") (OtherComp :type "PrimitiveComponent Object Reference") (OtherBodyIndex :type Integer) (bFromSweep :type Boolean) (SweepResult :type "HitResult Structure (by ref)"))
  (bind _asthird_person_character (cast `/Game/ThirdPersonBP/Blueprints/ThirdPersonCharacter` OtherActor))
  (set `/Game/ThirdPersonBP/Blueprints/ThirdPersonCharacter.FireRange` (+ (`/Game/ThirdPersonBP/Blueprints/ThirdPersonCharacter.FireRange` _asthird_person_character) (250.0 0.0 0.0)) _asthird_person_character)
  (set `/Game/ThirdPersonBP/Blueprints/ThirdPersonCharacter.Heat` (- (`/Game/ThirdPersonBP/Blueprints/ThirdPersonCharacter.Heat` _asthird_person_character) 0.125) _asthird_person_character)
  (`self.K2_DestroyActor`))

(fn `UserConstructionScript`)