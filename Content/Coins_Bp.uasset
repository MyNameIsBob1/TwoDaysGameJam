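; Collectible coin pickup actor that spins in place and is collected when the third-person character touches it.
; Tick adds a speed-scaled, frame-rate-independent yaw to the actor's rotation.
; On Box overlap with a ThirdPersonCharacter, it increments that character's CoinsCount and the Coins total in GameInst_BP, then destroys itself.
; If the game instance cast fails, the coin remains after the character's count increases.
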(event `self.ReceiveTick`
  (params (DeltaSeconds :type "Float (single-precision)"))
  (bind (_returnvalue_roll _returnvalue_pitch _returnvalue_yaw) (`KismetMathLibrary.BreakRotator` (`self.K2_GetActorRotation`)))
  (`self.K2_SetActorRotation` (`KismetMathLibrary.MakeRotator` _returnvalue_roll _returnvalue_pitch (+ (* (`self.TrunSpeed`) DeltaSeconds) _returnvalue_yaw)) true))

(event `self.Box.OnComponentBeginOverlap`
  (params (OverlappedComponent :type "PrimitiveComponent Object Reference") (OtherActor :type "Actor Object Reference") (OtherComp :type "PrimitiveComponent Object Reference") (OtherBodyIndex :type Integer) (bFromSweep :type Boolean) (SweepResult :type "HitResult Structure (by ref)"))
  (bind _asthird_person_character (cast `/Game/ThirdPersonBP/Blueprints/ThirdPersonCharacter` OtherActor))
  (`/Engine/EditorBlueprintResources/StandardMacros.IncrementFloat` (`/Game/ThirdPersonBP/Blueprints/ThirdPersonCharacter.CoinsCount` _asthird_person_character)
    (:`  `
      (bind _asgame_inst_bp (cast `/Game/GameInst_BP` (`GameplayStatics.GetGameInstance`)))
      (`/Engine/EditorBlueprintResources/StandardMacros.IncrementFloat` (`/Game/GameInst_BP.Coins` _asgame_inst_bp)
        (:`  `
          (`self.K2_DestroyActor`))))))

(fn `UserConstructionScript`)